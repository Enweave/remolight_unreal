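; n8AppStorage handles persistent storage for the app through an n8SaveGame object held in Savedata.
; LoadState loads that object from the SlotName slot if a save exists, otherwise it creates a fresh one.
; SaveState writes Savedata back to the same slot, with both functions using user index 0.
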(fn `LoadState`
  (bind _returnvalue (`GameplayStatics.DoesSaveGameExist` (`self.slot_name`)))
  (if _returnvalue
    (bind _returnvalue_2 (`GameplayStatics.LoadGameFromSlot` (`self.slot_name`)))
    (bind _asn_8save_game (cast `/Game/Blueprints/n8SaveGame` _returnvalue_2))
    (set `self.save-data` _asn_8save_game)
    (else
      (bind _returnvalue_3 (`GameplayStatics.CreateSaveGameObject` "/Game/Blueprints/n8SaveGame.n8SaveGame_C"))
      (set `self.save-data` _returnvalue_3))))

(fn `SaveState`
  (`GameplayStatics.SaveGameToSlot` (`self.save-data`) (`self.slot_name`)))